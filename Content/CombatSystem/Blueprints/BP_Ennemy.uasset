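; Enemy combatant for the combat system that spawns with starting equipment, takes point damage and can be targeted until dead.
; On BeginPlay it initializes its stats component, then spawns and equips each starting item.
; Point damage feeds the stats component, plays sound and particles, and, when a hit reaction is allowed, sets the Disable state with a react montage.
; Tick prints one current stat as on-screen debug text.
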(event `self.ReceiveBeginPlay`
  (`/Game/CombatSystem/Blueprints/Components/BPC_StatsComponent.InitializaStats` (`self.BPC_StatsComponent`))
  (for _array_element (`self.StartEquipe`)
    (bind _returnvalue (`|SpawnActorFromClass` _array_element (`self.GetTransform`) "Undefined" "OverrideRootScale" self self))
    (`/Game/CombatSystem/Blueprints/Actors/BP_BaseEquippable.EquipeOnBody` _returnvalue)))

(event `self.ReceiveTick`
  (params (DeltaSeconds :type "Float (single-precision)"))
  (`parent.ReceiveTick` DeltaSeconds)
  (`KismetSystemLibrary.PrintString` (`KismetStringLibrary.Conv_DoubleToString` (`/Game/CombatSystem/Blueprints/Components/BPC_StatsComponent.GetCurrentStatValue` (`self.BPC_StatsComponent`) "NewEnumerator4")) true true (struct :`R` 1.0 :`G` 0.11875 :`A` 1.0) 0.001))

(event `self.ReceivePointDamage`
  (params (Damage :type "Float (single-precision)") (DamageType :type "DamageType Object Reference") (HitLocation :type "Vector Structure") (HitNormal :type "Vector Structure") (HitComponent :type "PrimitiveComponent Object Reference") (BoneName :type Name) (ShotFromDirection :type "Vector Structure") (InstigatedBy :type "Controller Object Reference") (DamageCauser :type "Actor Object Reference") (HitInfo :type "HitResult Structure (by ref)"))
  (`/Game/CombatSystem/Blueprints/Components/BPC_StatsComponent.TakeDamage` (`self.BPC_StatsComponent`) Damage)
  (`GameplayStatics.PlaySoundAtLocation` "/Game/CombatSystem/Asset/SoundFX/Weapon/A_Sword_Swing_Cue.A_Sword_Swing_Cue" HitLocation (struct) 1.0 1.0 0.0 null null null null)
  (`GameplayStatics.SpawnEmitterAtLocation` null HitLocation)
  (if (`self.CanReceiveHitReaction?`)
    (`/Game/CombatSystem/Blueprints/Components/BPC_StateManagerComponent.SetCurrentState` (`self.BPC_StateManagerComponent`) (struct :`TagName` "Character.State.Disable"))
    (`self.PlayAnimMontage` "/Game/Characters/UE4_MannyAnim/Standing_React_Large_Front_Montage.Standing_React_Large_Front_Montage")))

(event `/Game/CombatSystem/Blueprints/Interface/BPI_Targeting.OnTargeted`
  (params (isTargeted :type Boolean)))

(fn `CanBeTargeted?`
  (returns (`CanBeTargetrd?` :type Boolean))
  (return (not (`/Game/CombatSystem/Blueprints/Components/BPC_StateManagerComponent.IsCurrentStateEqualTo?` (`self.BPC_StateManagerComponent`) (struct :`GameplayTags` (struct :`(TagName` "Character.State.Dead")))))))

(fn `UserConstructionScript`
  (`parent.UserConstructionScript`))