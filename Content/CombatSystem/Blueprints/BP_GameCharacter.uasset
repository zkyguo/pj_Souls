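; Combat character Blueprint that handles attacks, dodges, weapon draw and disarm, movement speeds, damage and death.
; State manager, combat and stats components drive it, with gameplay-tag states gating actions and the main weapon supplying montages.
; Normal attacks cycle by combo count or pick randomly, while point damage feeds stats and triggers hit reactions.
; Death ragdolls the mesh with a backward impulse, drops the weapon and destroys both after a delay.
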(event `self.ReceiveBeginPlay`
  ;[1 1 1] Begin Play
)

(event `/Game/CombatSystem/Blueprints/Interface/BPI_Combat.ResetCombat`
  (bind _bpc_statemanagercomponent (`self.BPC_StateManagerComponent`))
  (bind _mainweapon (`/Game/CombatSystem/Blueprints/Components/BPC_CombatComponent.GetMainWeapon` (`self.BPC_CombatComponent`)))
  ;[1 1 1] Combat interface
  (`/Engine/EditorBlueprintResources/StandardMacros.IsValid` _mainweapon
    (:`Is Valid`
      (`/Game/CombatSystem/Blueprints/Components/BPC_StateManagerComponent.ResetState` _bpc_statemanagercomponent (`/Game/CombatSystem/Blueprints/Actors/BP_BaseWeapon.IsWeaponOnHand` _mainweapon)))
    (:`Is Not Valid`
      (`/Game/CombatSystem/Blueprints/Components/BPC_StateManagerComponent.SetCurrentState` _bpc_statemanagercomponent (struct :`TagName` "Character.State.None"))))
  (`/Game/CombatSystem/Blueprints/Components/BPC_StateManagerComponent.SetCurrentAction` _bpc_statemanagercomponent (struct :`TagName` "Character.Action.Nothing"))
  (set `/Game/CombatSystem/Blueprints/Components/BPC_CombatComponent.AttackCount` 0 (`self.BPC_CombatComponent`)))

(event `/Game/CombatSystem/Blueprints/Interface/BPI_Combat.ResetAttack`
  ;[1 1 1] Combat interface
  (`/Game/CombatSystem/Blueprints/Components/BPC_StateManagerComponent.SetCurrentState` (`self.BPC_StateManagerComponent`) (struct :`TagName` "Character.State.General Action")))

(event `/Game/CombatSystem/Blueprints/Interface/BPI_Combat.ResetAttackIndex`
  ;[1 1 1] Combat interface
  (set `/Game/CombatSystem/Blueprints/Components/BPC_CombatComponent.AttackCount` 0 (`self.BPC_CombatComponent`)))

(event `PerformDead`
  (bind _mainweapon (`/Game/CombatSystem/Blueprints/Components/BPC_CombatComponent.GetMainWeapon` (`self.BPC_CombatComponent`)))
  ;[1 1 1] Perform Dead
  (`self.EnableRagdoll`)
  (`self.ApplyHitReactionPhysicVelocity` -2000.0)
  (`|ExecutionSequence`
    (:`then_0`
      (`/Engine/EditorBlueprintResources/StandardMacros.IsValid` _mainweapon
        (:`Is Valid`
          (`/Game/CombatSystem/Blueprints/Actors/BP_BaseWeapon.SimulateWeaponPhysics` _mainweapon))))
    (:`then_1`
      (`KismetSystemLibrary.Delay` 4.0)
      (`/Engine/EditorBlueprintResources/StandardMacros.IsValid` _mainweapon
        (:`Is Valid`
          (`self.K2_DestroyActor` _mainweapon))
        (:`Is Not Valid`
          _))
      (`self.K2_DestroyActor`))))

(event `ApplyHitReaction`
  (params (`Damage Reaction` :type "/Game/CombatSystem/Blueprints/Enum/E_DamageReactionType Enum" :default "NewEnumerator0"))
  ;[1 1 1] Hit Reaction
  (switch `/Game/CombatSystem/Blueprints/Enum/E_DamageReactionType` `Damage Reaction`
    (:`NewEnumerator1`
      (`self.PerformKnockBack`))
    (:`NewEnumerator2`
      (`self.PerformHitStun`))))

(event `self.ReceivePointDamage`
  (params (Damage :type "Float (single-precision)") (DamageType :type "DamageType Object Reference") (HitLocation :type "Vector Structure") (HitNormal :type "Vector Structure") (HitComponent :type "PrimitiveComponent Object Reference") (BoneName :type Name) (ShotFromDirection :type "Vector Structure") (InstigatedBy :type "Controller Object Reference") (DamageCauser :type "Actor Object Reference") (HitInfo :type "HitResult Structure (by ref)"))
  ;[1 1 1] Hit Damage
  (`/Game/CombatSystem/Blueprints/Components/BPC_StatsComponent.TakeDamage` (`self.BPC_StatsComponent`) Damage)
  (set `self.HitDirection` (`self.GetDotProductTo` (`Controller.K2_GetPawn` InstigatedBy) self))
  (`GameplayStatics.PlaySoundAtLocation` "/Game/CombatSystem/Asset/SoundFX/Weapon/A_Sword_Swing_Cue.A_Sword_Swing_Cue" HitLocation (struct) 1.0 1.0 0.0 null null null null)
  (`GameplayStatics.SpawnEmitterAtLocation` null HitLocation)
  (if (`self.CanReceiveHitReaction?`)
    (`/Game/CombatSystem/Blueprints/Components/BPC_StateManagerComponent.SetCurrentState` (`self.BPC_StateManagerComponent`) (struct :`TagName` "Character.State.Disable"))
    (`self.PerformHitReaction`)))

(event `PerformHitReaction`
  (`self.PlayAnimMontage` "/Game/CombatSystem/Asset/Animations/HitReactions/Standing_React_Large_Front_Montage.Standing_React_Large_Front_Montage"))

(event `self.BPC_StateManagerComponent.OnStateBegin`
  (params (CharacterState :type "GameplayTag Structure"))
  ;[1 1 1] State Machine
  (`|SwitchGameplayTag` CharacterState
    (:`Character.State.Dead`
      (`self.PerformDead`))))

(event `self.BPC_StateManagerComponent.OnStateEnd`
  (params (CharacterState :type "GameplayTag Structure"))
  ;[1 1 1] State Machine
)

(event `self.BPC_StateManagerComponent.OnCharacterActionBegin`
  (params (Action :type "GameplayTag Structure"))
  ;[1 1 1] State Machine
)

(event `self.BPC_StateManagerComponent.OnCharacterActionEnd`
  (params (Action :type "GameplayTag Structure"))
  ;[1 1 1] State Machine
)

(fn `ApplyHitReactionPhysicVelocity`
  (params (InitialSpeed :type "Float (double-precision)"))
  (`PrimitiveComponent.SetPhysicsLinearVelocity` (`self.Mesh`) (* (`self.GetActorForwardVector`) (`local.InitialSpeed`)) false (`self.Pelvis Bone Name`)))

(fn `AttackTypeCheck`
  (returns (AttackType :type "GameplayTag Structure"))
  (if (`NavMovementComponent.IsFalling` (`self.CharacterMovement`))
    (return (struct :`TagName` "Character.Action.Attack.FallingAttack"))
    (elif (`|EnumEquality` (`self.MovementSpeedMode`) "NewEnumerator2")
      (return (struct :`TagName` "Character.Action.Attack.SprintAttack"))
      (else
        (return (struct :`TagName` "Character.Action.Attack.NormalAttack"))))))

(fn `Can Draw Disarm?`
  (returns (`CanDrawDisarm?` :type Boolean))
  (`/Engine/EditorBlueprintResources/StandardMacros.IsValid` (`/Game/CombatSystem/Blueprints/Components/BPC_CombatComponent.GetMainWeapon` (`self.BPC_CombatComponent`))
    (:`Is Valid`
      (return (and (not (`/Game/CombatSystem/Blueprints/Components/BPC_StateManagerComponent.IsCurrentStateEqualTo?` (`self.BPC_StateManagerComponent`) (struct :`GameplayTags` (struct :`(TagName` "Character.State.Attacking") :`(TagName` "Character.State.Dead") :`(TagName` "Character.State.Disable") :`(TagName` "Character.State.Dodging"))))) (not (`NavMovementComponent.IsFalling` (`self.CharacterMovement`))) (not (`AnimInstance.IsAnyMontagePlaying` (`SkeletalMeshComponent.GetAnimInstance` (`self.Mesh`)))))))))

(fn `CanJump?`
  (returns (`CanJump?` :type Boolean))
  (return (and (not (`/Game/CombatSystem/Blueprints/Components/BPC_StateManagerComponent.IsCurrentStateEqualTo?` (`self.BPC_StateManagerComponent`) (struct :`GameplayTags` (struct :`(TagName` "Character.State.Attacking") :`(TagName` "Character.State.Dead") :`(TagName` "Character.State.Disable") :`(TagName` "Character.State.Dodging"))))) (not (`NavMovementComponent.IsFalling` (`self.CharacterMovement`))))))

(fn `CanReceiveDamage`
  (returns (`CanReceiveDamage?` :type Boolean))
  (return (not (`/Game/CombatSystem/Blueprints/Components/BPC_StateManagerComponent.IsCurrentStateEqualTo?` (`self.BPC_StateManagerComponent`) (struct :`GameplayTags` (struct :`(TagName` "Character.State.Dead") :`(TagName` "Character.State.Dodging")))))))

(fn `CanReceiveHitReaction?`
  (returns (`CanReceive?` :type Boolean))
  (return (!= (`/Game/CombatSystem/Blueprints/Components/BPC_StateManagerComponent.GetCurrentState` (`self.BPC_StateManagerComponent`)) (struct :`TagName` "Character.State.Dead"))))

(fn `DrawWeapon`
  (bind _mainweapon (`/Game/CombatSystem/Blueprints/Components/BPC_CombatComponent.GetMainWeapon` (`self.BPC_CombatComponent`)))
  (bind _candrawdisarm_ (`self.Can Draw Disarm?`))
  (if _candrawdisarm_
    (if (`/Game/CombatSystem/Blueprints/Actors/BP_BaseWeapon.IsWeaponOnHand` _mainweapon)
      (bind _equipemontage (`/Game/CombatSystem/Blueprints/Actors/BP_BaseWeapon.Find Weapon Montage` _mainweapon (struct :`TagName` "Character.Action.DisarmWeapon")))
      (`self.PlayAnimMontage` (`|GetArrayItem` _equipemontage))
      (else
        (bind _equipemontage_2 (`/Game/CombatSystem/Blueprints/Actors/BP_BaseWeapon.Find Weapon Montage` _mainweapon (struct :`TagName` "Character.Action.DrawWeapon")))
        (`self.PlayAnimMontage` (`|GetArrayItem` _equipemontage_2))))))

(fn `EnableRagdoll`
  (bind _mesh (`self.Mesh`))
  (bind _pelvis_bone_name (`self.Pelvis Bone Name`))
  (bind _cameraboom (`self.CameraBoom`))
  (bind _capsulecomponent (`self.CapsuleComponent`))
  (`CharacterMovementComponent.SetMovementMode` (`self.CharacterMovement`) "MOVE_None" 0) ; Disable movement
  (`PrimitiveComponent.SetCollisionResponseToChannel` _capsulecomponent "ECC_Pawn" "ECR_Ignore") ; Disable mesh collision capsule
  (`PrimitiveComponent.SetCollisionResponseToChannel` _capsulecomponent "ECC_Camera" "ECR_Ignore") ; Disable Camera collision capsule
  (`SceneComponent.K2_AttachToComponent` _cameraboom (`self.Mesh`) (`self.Pelvis Bone Name`) "KeepWorld" "KeepWorld" "KeepWorld" true)
  (set `SpringArmComponent.bDoCollisionTest` false _cameraboom)
  (`PrimitiveComponent.SetCollisionProfileName` (`self.Mesh`) "ragdoll" true)
  (`SkeletalMeshComponent.SetAllBodiesBelowSimulatePhysics` _mesh _pelvis_bone_name true true)
  (`SkeletalMeshComponent.SetAllBodiesBelowPhysicsBlendWeight` _mesh _pelvis_bone_name 1.0 false true))

(fn `GetDesiredRotation`
  (returns (ReturnValue :type "Rotator Structure"))
  (if (!= (`PawnMovementComponent.GetLastInputVector` (`self.CharacterMovement`)) (0.0 0.0 0.0) :`ErrorTolerance` 0.0001)
    (return (`KismetMathLibrary.Conv_VectorToRotator` (`self.GetLastMovementInputVector`)))
    (else
      (return (`self.K2_GetActorRotation`)))))

(fn `GetMovementSpeedMode`
  (returns (`Current Mode` :type "/Game/CombatSystem/Blueprints/Enum/E_MovementSpeed Enum"))
  (return (`self.MovementSpeedMode`)))

(fn `GetOwnerGamePlayTag`
  (returns (tag :type "GameplayTag Structure"))
  (return))

(fn `HasMatchingGameplayTag`
  (params (Tag :type "GameplayTag Structure"))
  (returns (`isMatching?` :type Boolean))
  (return (`BlueprintGameplayTagLibrary.HasTag` (`self.OwnTag`) Tag)))

(fn `Perform Combat Action`
  (params (ActionTag :type "GameplayTag Structure") (StateTag :type "GameplayTag Structure") (MontageIndex :type Integer) (`RandomIndex?` :type Boolean))
  (returns (ActionDuraction :type "Float (double-precision)"))
  (return 0.0))

(fn `Perform Combat Attack`
  (params (AttackType :type "GameplayTag Structure") (AttackIndex :type Integer) (`RandomIndex?` :type Boolean))
  (returns (AttackDuration :type "Float (double-precision)"))
  (return 0.0))

(fn `Perform Dodge`
  (params (DodgeIndex :type Integer))
  (locals (DodgeMontage :type "AnimMontage Object Reference"))
  (bind _bpc_statemanagercomponent (`self.BPC_StateManagerComponent`))
  (bind _mainweapon (`/Game/CombatSystem/Blueprints/Components/BPC_CombatComponent.GetMainWeapon` (`self.BPC_CombatComponent`)))
  (`/Engine/EditorBlueprintResources/StandardMacros.IsValid` _mainweapon
    (:`Is Valid`
      (bind _output_get (set `local.DodgeMontage` (`|GetArrayItem` (`/Game/CombatSystem/Blueprints/Actors/BP_BaseWeapon.DodgeMontage` _mainweapon) DodgeIndex)))
      (`/Engine/EditorBlueprintResources/StandardMacros.IsValid` _output_get
        (:`Is Valid`
          (`/Game/CombatSystem/Blueprints/Components/BPC_StateManagerComponent.SetCurrentState` _bpc_statemanagercomponent (struct :`TagName` "Character.State.Dodging"))
          (`/Game/CombatSystem/Blueprints/Components/BPC_StateManagerComponent.SetCurrentAction` _bpc_statemanagercomponent (struct :`TagName` "Character.Action.Dodge"))
          (`self.PlayAnimMontage` (`local.DodgeMontage`)))))
    (:`Is Not Valid`
      (`/Game/CombatSystem/Blueprints/Components/BPC_StateManagerComponent.SetCurrentState` _bpc_statemanagercomponent (struct :`TagName` "Character.State.Dodging"))
      (`/Game/CombatSystem/Blueprints/Components/BPC_StateManagerComponent.SetCurrentAction` _bpc_statemanagercomponent (struct :`TagName` "Character.Action.Dodge"))
      (`self.PlayAnimMontage` "/Game/CombatSystem/Asset/Animations/Dodge/Rolling_Montage.Rolling_Montage"))))

(fn `PerformAttack`
  (params (AttackIndex :type Integer) (`RandomIndex?` :type Boolean) (AttackType :type "GameplayTag Structure"))
  (returns (`Attack Duration` :type "Float (single-precision)"))
  (bind _bpc_combatcomponent (`self.BPC_CombatComponent`))
  (`|SwitchGameplayTag` AttackType
    (:`Character.Action.Attack.NormalAttack`
      (bind _equipemontage (`/Game/CombatSystem/Blueprints/Actors/BP_BaseWeapon.Find Weapon Montage` (`/Game/CombatSystem/Blueprints/Components/BPC_CombatComponent.GetMainWeapon` (`self.BPC_CombatComponent`)) (struct :`TagName` "Character.Action.Attack.NormalAttack")))
      (bind _output_get (set `self.AttackMontage` (select `bool` (`local.RandomIndex?`) :`false` (`|GetArrayItem` _equipemontage (`local.AttackIndex`)) :`true` (`KismetArrayLibrary.Array_Random` _equipemontage))))
      (`/Engine/EditorBlueprintResources/StandardMacros.IsValid` _output_get
        (:`Is Valid`
          (`/Game/CombatSystem/Blueprints/Components/BPC_StateManagerComponent.SetCurrentState` (`self.BPC_StateManagerComponent`) (struct :`TagName` "Character.State.Attacking"))
          (`/Game/CombatSystem/Blueprints/Components/BPC_StateManagerComponent.SetCurrentAction` (`self.BPC_StateManagerComponent`) (struct :`TagName` "Character.Action.Attack.NormalAttack"))
          (bind _returnvalue (`self.PlayAnimMontage` (`self.AttackMontage`)))
          (bind _result (`/Engine/EditorBlueprintResources/StandardMacros.IncrementInt` (`/Game/CombatSystem/Blueprints/Components/BPC_CombatComponent.AttackCount` _bpc_combatcomponent))
            (:`  `
              (bind _output_get_2 (set `/Game/CombatSystem/Blueprints/Components/BPC_CombatComponent.AttackCount` _result _bpc_combatcomponent))
              (if (> _output_get_2 (`KismetArrayLibrary.Array_LastIndex` _equipemontage))
                (set `/Game/CombatSystem/Blueprints/Components/BPC_CombatComponent.AttackCount` 0 _bpc_combatcomponent)
                (return _returnvalue)))))))
    (:`Character.Action.Attack.SpecialAttack`
      (bind _equipemontage_2 (`/Game/CombatSystem/Blueprints/Actors/BP_BaseWeapon.Find Weapon Montage` (`/Game/CombatSystem/Blueprints/Components/BPC_CombatComponent.GetMainWeapon` (`self.BPC_CombatComponent`)) (struct :`TagName` "Character.Action.Attack.SpecialAttack")))
      (bind _output_get_3 (set `self.AttackMontage` (`|GetArrayItem` _equipemontage_2)))
      (`/Game/CombatSystem/Blueprints/Components/BPC_StateManagerComponent.SetCurrentState` (`self.BPC_StateManagerComponent`) (struct :`TagName` "Character.State.Attacking"))
      (`/Game/CombatSystem/Blueprints/Components/BPC_StateManagerComponent.SetCurrentAction` (`self.BPC_StateManagerComponent`) (struct :`TagName` "Character.Action.Attack.SpecialAttack"))
      (`self.PlayAnimMontage` _output_get_3))))

(fn `PerformHitStun`
  (`/Game/CombatSystem/Blueprints/Components/BPC_StateManagerComponent.SetCurrentState` (`self.BPC_StateManagerComponent`) (struct :`TagName` "Character.State.Disable"))
  (`self.PlayAnimMontage` null))

(fn `PerformKnockBack`
  (`/Game/CombatSystem/Blueprints/Components/BPC_StateManagerComponent.SetCurrentState` (`self.BPC_StateManagerComponent`) (struct :`TagName` "Character.State.Disable"))
  (`self.PlayAnimMontage` "/Game/Characters/UE4_MannyAnim/Standing_React_Large_Front_Montage.Standing_React_Large_Front_Montage"))

(fn `SetMovementSpeedMode`
  (params (NewSpeedMode :type "/Game/CombatSystem/Blueprints/Enum/E_MovementSpeed Enum" :default "NewEnumerator0"))
  (bind _charactermovement (`self.CharacterMovement`))
  (if (`|EnumInequality` NewSpeedMode (`self.MovementSpeedMode`))
    (bind _output_get (set `self.MovementSpeedMode` NewSpeedMode))
    (switch `/Game/CombatSystem/Blueprints/Enum/E_MovementSpeed` _output_get
      (:`NewEnumerator0`
        (set `CharacterMovementComponent.MaxWalkSpeed` 200.0 _charactermovement))
      (:`NewEnumerator1`
        (set `CharacterMovementComponent.MaxWalkSpeed` 450.0 _charactermovement))
      (:`NewEnumerator2`
        (set `CharacterMovementComponent.MaxWalkSpeed` 700.0 _charactermovement)))))

(fn `UserConstructionScript`)