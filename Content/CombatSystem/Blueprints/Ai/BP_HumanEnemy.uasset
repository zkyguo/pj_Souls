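; Human enemy AI character Blueprint that adds a health bar display on top of its parent enemy behavior.
; On BeginPlay it creates a health bar widget bound to its EnemyStats component, assigns it to the HealthBar widget component and hides it.
; The targeting event toggles the bar, so it is visible only while the enemy is targeted.
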(event `self.ReceiveBeginPlay`
  (bind _healthbar (`self.HealthBar`))
  (`parent.ReceiveBeginPlay`)
  (bind _returnvalue (`|CreateWidget` "/Game/CombatSystem/Blueprints/UI/WB_HealthBar.WB_HealthBar_C" (`GameplayStatics.GetPlayerController` 0) (`self.Enemy Stats`)))
  (`WidgetComponent.SetWidget` _healthbar _returnvalue)
  (`SceneComponent.SetVisibility` _healthbar false false))

(event `/Game/CombatSystem/Blueprints/Interface/BPI_Targeting.OnTargeted`
  (params (isTargeted :type Boolean))
  (`parent.OnTargeted` isTargeted)
  (`SceneComponent.SetVisibility` (`self.HealthBar`) isTargeted false))

(fn `UserConstructionScript`
  (`parent.UserConstructionScript`))