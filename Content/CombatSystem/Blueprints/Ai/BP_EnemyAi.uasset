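; Enemy combat character with attacks, dodges, weapon draw, hit reactions and lock-on targeting, triggered here by input-action events rather than AI logic.
; State manager gameplay tags and stat checks gate actions, which play montages mostly taken from the combat component's main weapon.
; Point damage feeds EnemyStats, spawns effects and triggers hit reactions.
; Death ragdolls the body with a backward shove, drops the weapon and destroys both after a delay.
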(event `self.ReceiveBeginPlay`
  (`/Game/CombatSystem/Blueprints/Components/BPC_StatsComponent.InitializaStats` (`self.Enemy Stats`)))

(event `InputAction|ToggleCombat`
  (params (Key :type "Key Structure"))
  ;[1 1 1] Draw/Disarm Weapon
  (:`Pressed`
    (`self.DrawWeapon`)))

(event `PerformDead`
  (bind _mainweapon (`/Game/CombatSystem/Blueprints/Components/BPC_CombatComponent.GetMainWeapon` (`self.BPC_CombatComponent`)))
  ;[1 1 1] Perform Dead
  (`self.EnableRagdoll`)
  (`self.ApplyHitReactionPhysicVelocity` -2000.0)
  (`|ExecutionSequence`
    (:`then_0`
      (`/Engine/EditorBlueprintResources/StandardMacros.IsValid` _mainweapon
        (:`Is Valid`
          (`/Game/CombatSystem/Blueprints/Actors/BP_BaseWeapon.SimulateWeaponPhysics` _mainweapon))))
    (:`then_1`
      (`KismetSystemLibrary.Delay` 4.0)
      (`/Engine/EditorBlueprintResources/StandardMacros.IsValid` _mainweapon
        (:`Is Valid`
          (`self.K2_DestroyActor` _mainweapon))
        (:`Is Not Valid`
          _))
      (`self.K2_DestroyActor`))))

(event `InputAction|NormalAttack`
  (params (Key :type "Key Structure"))
  ;[1 1 1] Normal Attack
  (:`Pressed`
    (if (`self.CanAttack?`)
      (bind _attacktype (`self.AttackTypeCheck`))
      (`self.PerformAttack` 0 true _attacktype))))

(event `InputAction|Dodge`
  (params (Key :type "Key Structure"))
  ;[1 1 1] Dodge
  (:`Pressed`
    (if (`self.CanDodge?`)
      (`self.Perform Dodge` 0))))

(event `self.BPC_StateManagerComponent.OnStateBegin`
  (params (CharacterState :type "GameplayTag Structure"))
  ;[1 1 1] Character State Machine
  (`|SwitchGameplayTag` CharacterState
    (:`Character.State.Dead`
      (`self.PerformDead`))))

(event `InputAction|SpecialAttack`
  (params (Key :type "Key Structure"))
  ;[1 1 1] Special Attack
  (:`Pressed`
    (if (`self.CanAttack?`)
      (`self.PerformAttack` 0 false "NewEnumerator1"))))

(event `ApplyHitReaction`
  (params (`Damage Reaction` :type "/Game/CombatSystem/Blueprints/Enum/E_DamageReactionType Enum" :default "NewEnumerator0"))
  ;[1 1 1] Hit Reaction
  (switch `/Game/CombatSystem/Blueprints/Enum/E_DamageReactionType` `Damage Reaction`
    (:`NewEnumerator1`
      (`self.PerformKnockBack`))
    (:`NewEnumerator2`
      (`self.PerformHitStun`))))

(event `self.BPC_StateManagerComponent.OnStateEnd`
  (params (CharacterState :type "GameplayTag Structure"))
  ;[1 1 1] Character State Machine
)

(event `self.BPC_StateManagerComponent.OnCharacterActionBegin`
  (params (Action :type "GameplayTag Structure"))
  ;[1 1 1] Character Action
)

(event `self.ReceivePointDamage`
  (params (Damage :type "Float (single-precision)") (DamageType :type "DamageType Object Reference") (HitLocation :type "Vector Structure") (HitNormal :type "Vector Structure") (HitComponent :type "PrimitiveComponent Object Reference") (BoneName :type Name) (ShotFromDirection :type "Vector Structure") (InstigatedBy :type "Controller Object Reference") (DamageCauser :type "Actor Object Reference") (HitInfo :type "HitResult Structure (by ref)"))
  ;[1 1 1] Hit Damage
  (`/Game/CombatSystem/Blueprints/Components/BPC_StatsComponent.TakeDamage` (`self.Enemy Stats`) Damage)
  (`AISense_Damage.ReportDamageEvent` self (`Controller.K2_GetPawn` InstigatedBy) Damage HitLocation HitLocation)
  (`GameplayStatics.PlaySoundAtLocation` "/Game/CombatSystem/Asset/SoundFX/Weapon/A_Sword_Swing_Cue.A_Sword_Swing_Cue" HitLocation (struct) 1.0 1.0 0.0 null null null null)
  (`GameplayStatics.SpawnEmitterAtLocation` null HitLocation)
  (if (`self.CanReceiveHitReaction?`)
    (`/Game/CombatSystem/Blueprints/Components/BPC_StateManagerComponent.SetCurrentState` (`self.BPC_StateManagerComponent`) (struct :`TagName` "Character.State.Disable"))
    (`self.PerformHitReaction`)))

(event `self.BPC_StateManagerComponent.OnCharacterActionEnd`
  (params (Action :type "GameplayTag Structure"))
  ;[1 1 1] Character Action
)

(event `InputAction|Sprint`
  (params (Key :type "Key Structure"))
  ;[1 1 1] Movement speed mode
  (:`Pressed`
    (`self.SetMovementSpeedMode` "NewEnumerator2"))
  (:`Released`
    (`self.SetMovementSpeedMode` "NewEnumerator1")))

(event `InputAction|ToggleWalking`
  (params (Key :type "Key Structure"))
  ;[1 1 1] Movement speed mode
  (:`Pressed`
    (`self.SetMovementSpeedMode` "NewEnumerator0"))
  (:`Released`
    (`self.SetMovementSpeedMode` "NewEnumerator1")))

(event `/Game/CombatSystem/Blueprints/Interface/BPI_Combat.ResetCombat`
  (bind _bpc_statemanagercomponent (`self.BPC_StateManagerComponent`))
  (bind _mainweapon (`/Game/CombatSystem/Blueprints/Components/BPC_CombatComponent.GetMainWeapon` (`self.BPC_CombatComponent`)))
  ;[1 1 1] Combat interface
  (`/Engine/EditorBlueprintResources/StandardMacros.IsValid` _mainweapon
    (:`Is Valid`
      (`/Game/CombatSystem/Blueprints/Components/BPC_StateManagerComponent.ResetState` _bpc_statemanagercomponent (`/Game/CombatSystem/Blueprints/Actors/BP_BaseWeapon.IsWeaponOnHand` _mainweapon)))
    (:`Is Not Valid`
      (`/Game/CombatSystem/Blueprints/Components/BPC_StateManagerComponent.SetCurrentState` _bpc_statemanagercomponent (struct :`TagName` "Character.State.None"))))
  (`/Game/CombatSystem/Blueprints/Components/BPC_StateManagerComponent.SetCurrentAction` _bpc_statemanagercomponent (struct :`TagName` "Character.Action.Nothing"))
  (set `/Game/CombatSystem/Blueprints/Components/BPC_CombatComponent.AttackCount` 0 (`self.BPC_CombatComponent`)))

(event `/Game/CombatSystem/Blueprints/Interface/BPI_Combat.ResetAttack`
  ;[1 1 1] Combat interface
  (`/Game/CombatSystem/Blueprints/Components/BPC_StateManagerComponent.SetCurrentState` (`self.BPC_StateManagerComponent`) (struct :`TagName` "Character.State.General Action")))

(event `PerformHitReaction`
  (`self.PlayAnimMontage` "/Game/CombatSystem/Asset/Animations/HitReactions/Standing_React_Large_Front_Montage.Standing_React_Large_Front_Montage"))

(event `/Game/CombatSystem/Blueprints/Interface/BPI_Combat.ResetAttackIndex`
  ;[1 1 1] Combat interface
  (set `/Game/CombatSystem/Blueprints/Components/BPC_CombatComponent.AttackCount` 0 (`self.BPC_CombatComponent`)))

(event `/Game/CombatSystem/Blueprints/Interface/BPI_Targeting.OnTargeted`
  (params (isTargeted :type Boolean))
  ;[1 1 1] if actor is on target
  (`SceneComponent.SetVisibility` (`self.LockOnWidget`) isTargeted false))

(fn `ApplyHitReactionPhysicVelocity`
  (params (InitialSpeed :type "Float (double-precision)"))
  (`PrimitiveComponent.SetPhysicsLinearVelocity` (`self.Mesh`) (* (`self.GetActorForwardVector`) (`local.InitialSpeed`)) false (`self.Pelvis Bone Name`)))

(fn `AttackTypeCheck`
  (returns (AttackType :type "/Game/CombatSystem/Blueprints/Enum/E_CharacterAction Enum"))
  (if (`NavMovementComponent.IsFalling` (`self.CharacterMovement`))
    (return "NewEnumerator3")
    (elif (`|EnumEquality` (`self.MovementSpeedMode`) "NewEnumerator2")
      (return "NewEnumerator9")
      (else
        (return "NewEnumerator0")))))

(fn `Can Draw Disarm?`
  (returns (`CanDrawDisarm?` :type Boolean))
  (`/Engine/EditorBlueprintResources/StandardMacros.IsValid` (`/Game/CombatSystem/Blueprints/Components/BPC_CombatComponent.GetMainWeapon` (`self.BPC_CombatComponent`))
    (:`Is Valid`
      (return (and (not (`/Game/CombatSystem/Blueprints/Components/BPC_StateManagerComponent.IsCurrentStateEqualTo?` (`self.BPC_StateManagerComponent`) (struct :`GameplayTags` (struct :`(TagName` "Character.State.Attacking") :`(TagName` "Character.State.Dead") :`(TagName` "Character.State.Disable") :`(TagName` "Character.State.Dodging"))))) (not (`NavMovementComponent.IsFalling` (`self.CharacterMovement`))) (not (`AnimInstance.IsAnyMontagePlaying` (`SkeletalMeshComponent.GetAnimInstance` (`self.Mesh`)))))))))

(fn `CanAttack?`
  (returns (`CanAttack?` :type Boolean))
  (`/Engine/EditorBlueprintResources/StandardMacros.IsValid` (`/Game/CombatSystem/Blueprints/Components/BPC_CombatComponent.GetMainWeapon` (`self.BPC_CombatComponent`))
    (:`Is Valid`
      (return (and (not (`/Game/CombatSystem/Blueprints/Components/BPC_StateManagerComponent.IsCurrentStateEqualTo?` (`self.BPC_StateManagerComponent`) (struct :`GameplayTags` (struct :`(TagName` "Character.State.Attacking") :`(TagName` "Character.State.Dead") :`(TagName` "Character.State.Disable") :`(TagName` "Character.State.Dodging") :`(TagName` "Character.State.None"))))) (>= (`/Game/CombatSystem/Blueprints/Components/BPC_StatsComponent.GetCurrentStatValue` (`self.Enemy Stats`) "NewEnumerator2") 10.0))))))

(fn `CanBeTargeted?`
  (returns (`CanBeTargetrd?` :type Boolean))
  (return (!= (`/Game/CombatSystem/Blueprints/Components/BPC_StateManagerComponent.GetCurrentState` (`self.BPC_StateManagerComponent`)) (struct :`TagName` "Character.State.Dead"))))

(fn `CanDodge?`
  (returns (`CanDodge?` :type Boolean))
  (return (and (not (`NavMovementComponent.IsFalling` (`self.CharacterMovement`))) (not (`/Game/CombatSystem/Blueprints/Components/BPC_StateManagerComponent.IsCurrentStateEqualTo?` (`self.BPC_StateManagerComponent`) (struct :`GameplayTags` (struct :`(TagName` "Character.State.Attacking") :`(TagName` "Character.State.Dead") :`(TagName` "Character.State.Disable"))))) (>= (`/Game/CombatSystem/Blueprints/Components/BPC_StatsComponent.GetCurrentStatValue` (`self.Enemy Stats`) "NewEnumerator2") 10.0))))

(fn `CanJump?`
  (returns (`CanJump?` :type Boolean))
  (return (and (not (`/Game/CombatSystem/Blueprints/Components/BPC_StateManagerComponent.IsCurrentStateEqualTo?` (`self.BPC_StateManagerComponent`) (struct :`GameplayTags` (struct :`(TagName` "Character.State.Attacking") :`(TagName` "Character.State.Dead") :`(TagName` "Character.State.Disable") :`(TagName` "Character.State.Dodging"))))) (not (`NavMovementComponent.IsFalling` (`self.CharacterMovement`))))))

(fn `CanReceiveDamage`
  (returns (`CanReceiveDamage?` :type Boolean))
  (return (not (`/Game/CombatSystem/Blueprints/Components/BPC_StateManagerComponent.IsCurrentStateEqualTo?` (`self.BPC_StateManagerComponent`) (struct :`GameplayTags` (struct :`(TagName` "Character.State.Dead") :`(TagName` "Character.State.Dodging")))))))

(fn `CanReceiveHitReaction?`
  (returns (`CanReceive?` :type Boolean))
  (return (!= (`/Game/CombatSystem/Blueprints/Components/BPC_StateManagerComponent.GetCurrentState` (`self.BPC_StateManagerComponent`)) (struct :`TagName` "Character.State.Dead"))))

(fn `DrawWeapon`
  (bind _mainweapon (`/Game/CombatSystem/Blueprints/Components/BPC_CombatComponent.GetMainWeapon` (`self.BPC_CombatComponent`)))
  (bind _candrawdisarm_ (`self.Can Draw Disarm?`))
  (if _candrawdisarm_
    (if (`/Game/CombatSystem/Blueprints/Actors/BP_BaseWeapon.IsWeaponOnHand` _mainweapon)
      (bind _equipemontage (`/Game/CombatSystem/Blueprints/Actors/BP_BaseWeapon.Find Weapon Montage` _mainweapon (struct :`TagName` "Character.Action.DisarmWeapon")))
      (`self.PlayAnimMontage` (`|GetArrayItem` _equipemontage))
      (else
        (bind _equipemontage_2 (`/Game/CombatSystem/Blueprints/Actors/BP_BaseWeapon.Find Weapon Montage` _mainweapon (struct :`TagName` "Character.Action.DrawWeapon")))
        (`self.PlayAnimMontage` (`|GetArrayItem` _equipemontage_2))))))

(fn `EnableRagdoll`
  (bind _mesh (`self.Mesh`))
  (bind _pelvis_bone_name (`self.Pelvis Bone Name`))
  (bind _capsulecomponent (`self.CapsuleComponent`))
  (`CharacterMovementComponent.SetMovementMode` (`self.CharacterMovement`) "MOVE_None" 0) ; Disable movement
  (`PrimitiveComponent.SetCollisionResponseToChannel` _capsulecomponent "ECC_Pawn" "ECR_Ignore") ; Disable mesh collision capsule
  (`PrimitiveComponent.SetCollisionResponseToChannel` _capsulecomponent "ECC_Camera" "ECR_Ignore") ; Disable Camera collision capsule
  (`PrimitiveComponent.SetCollisionProfileName` (`self.Mesh`) "ragdoll" true)
  (`SkeletalMeshComponent.SetAllBodiesBelowSimulatePhysics` _mesh _pelvis_bone_name true true)
  (`SkeletalMeshComponent.SetAllBodiesBelowPhysicsBlendWeight` _mesh _pelvis_bone_name 1.0 false true))

(fn `GetDesiredRotation`
  (returns (ReturnValue :type "Rotator Structure"))
  (if (!= (`PawnMovementComponent.GetLastInputVector` (`self.CharacterMovement`)) (0.0 0.0 0.0) :`ErrorTolerance` 0.0001)
    (return (`KismetMathLibrary.Conv_VectorToRotator` (`self.GetLastMovementInputVector`)))
    (else
      (return (`self.K2_GetActorRotation`)))))

(fn `GetMovementSpeedMode`
  (returns (`Current Mode` :type "/Game/CombatSystem/Blueprints/Enum/E_MovementSpeed Enum"))
  (return (`self.MovementSpeedMode`)))

(fn `Perform Dodge`
  (params (DodgeIndex :type Integer))
  (locals (DodgeMontage :type "AnimMontage Object Reference"))
  (bind _bpc_statemanagercomponent (`self.BPC_StateManagerComponent`))
  (bind _mainweapon (`/Game/CombatSystem/Blueprints/Components/BPC_CombatComponent.GetMainWeapon` (`self.BPC_CombatComponent`)))
  (`/Engine/EditorBlueprintResources/StandardMacros.IsValid` _mainweapon
    (:`Is Valid`
      (bind _output_get (set `local.DodgeMontage` (`|GetArrayItem` (`/Game/CombatSystem/Blueprints/Actors/BP_BaseWeapon.DodgeMontage` _mainweapon) DodgeIndex)))
      (`/Engine/EditorBlueprintResources/StandardMacros.IsValid` _output_get
        (:`Is Valid`
          (`/Game/CombatSystem/Blueprints/Components/BPC_StateManagerComponent.SetCurrentState` _bpc_statemanagercomponent (struct :`TagName` "Character.State.Dodging"))
          (`/Game/CombatSystem/Blueprints/Components/BPC_StateManagerComponent.SetCurrentAction` _bpc_statemanagercomponent (struct :`TagName` "Character.Action.Dodge"))
          (`self.PlayAnimMontage` (`local.DodgeMontage`)))))
    (:`Is Not Valid`
      (`/Game/CombatSystem/Blueprints/Components/BPC_StateManagerComponent.SetCurrentState` _bpc_statemanagercomponent (struct :`TagName` "Character.State.Dodging"))
      (`/Game/CombatSystem/Blueprints/Components/BPC_StateManagerComponent.SetCurrentAction` _bpc_statemanagercomponent (struct :`TagName` "Character.Action.Dodge"))
      (`self.PlayAnimMontage` "/Game/CombatSystem/Asset/Animations/Dodge/Rolling_Montage.Rolling_Montage"))))

(fn `PerformAttack`
  (params (AttackIndex :type Integer) (`RandomIndex?` :type Boolean) (AttackType :type "/Game/CombatSystem/Blueprints/Enum/E_CharacterAction Enum" :default "NewEnumerator0"))
  (bind _bpc_combatcomponent (`self.BPC_CombatComponent`))
  (switch `/Game/CombatSystem/Blueprints/Enum/E_CharacterAction` AttackType
    (:`NewEnumerator0`
      (bind _equipemontage (`/Game/CombatSystem/Blueprints/Actors/BP_BaseWeapon.Find Weapon Montage` (`/Game/CombatSystem/Blueprints/Components/BPC_CombatComponent.GetMainWeapon` (`self.BPC_CombatComponent`)) (struct :`TagName` "Character.Action.Attack.NormalAttack")))
      (bind _output_get (set `self.AttackMontage` (select `bool` (`local.RandomIndex?`) :`false` (`|GetArrayItem` _equipemontage (`local.AttackIndex`)) :`true` (`KismetArrayLibrary.Array_Random` _equipemontage))))
      (`/Engine/EditorBlueprintResources/StandardMacros.IsValid` _output_get
        (:`Is Valid`
          (`/Game/CombatSystem/Blueprints/Components/BPC_StateManagerComponent.SetCurrentState` (`self.BPC_StateManagerComponent`) (struct :`TagName` "Character.State.Attacking"))
          (`/Game/CombatSystem/Blueprints/Components/BPC_StateManagerComponent.SetCurrentAction` (`self.BPC_StateManagerComponent`) (struct :`TagName` "Character.Action.Attack.NormalAttack"))
          (`self.PlayAnimMontage` (`self.AttackMontage`))
          (bind _result (`/Engine/EditorBlueprintResources/StandardMacros.IncrementInt` (`/Game/CombatSystem/Blueprints/Components/BPC_CombatComponent.AttackCount` _bpc_combatcomponent))
            (:`  `
              (bind _output_get_2 (set `/Game/CombatSystem/Blueprints/Components/BPC_CombatComponent.AttackCount` _result _bpc_combatcomponent))
              (if (> _output_get_2 (`KismetArrayLibrary.Array_LastIndex` _equipemontage))
                (set `/Game/CombatSystem/Blueprints/Components/BPC_CombatComponent.AttackCount` 0 _bpc_combatcomponent)))))))
    (:`NewEnumerator1`
      (bind _equipemontage_2 (`/Game/CombatSystem/Blueprints/Actors/BP_BaseWeapon.Find Weapon Montage` (`/Game/CombatSystem/Blueprints/Components/BPC_CombatComponent.GetMainWeapon` (`self.BPC_CombatComponent`)) (struct :`TagName` "Character.Action.Attack.SpecialAttack")))
      (bind _output_get_3 (set `self.AttackMontage` (`|GetArrayItem` _equipemontage_2)))
      (`/Game/CombatSystem/Blueprints/Components/BPC_StateManagerComponent.SetCurrentState` (`self.BPC_StateManagerComponent`) (struct :`TagName` "Character.State.Attacking"))
      (`/Game/CombatSystem/Blueprints/Components/BPC_StateManagerComponent.SetCurrentAction` (`self.BPC_StateManagerComponent`) (struct :`TagName` "Character.Action.Attack.SpecialAttack"))
      (`self.PlayAnimMontage` _output_get_3))))

(fn `PerformHitStun`
  (`/Game/CombatSystem/Blueprints/Components/BPC_StateManagerComponent.SetCurrentState` (`self.BPC_StateManagerComponent`) (struct :`TagName` "Character.State.Disable"))
  (`self.PlayAnimMontage` null))

(fn `PerformKnockBack`
  (`/Game/CombatSystem/Blueprints/Components/BPC_StateManagerComponent.SetCurrentState` (`self.BPC_StateManagerComponent`) (struct :`TagName` "Character.State.Disable"))
  (`self.PlayAnimMontage` "/Game/Characters/UE4_MannyAnim/Standing_React_Large_Front_Montage.Standing_React_Large_Front_Montage"))

(fn `SetMovementSpeedMode`
  (params (NewSpeedMode :type "/Game/CombatSystem/Blueprints/Enum/E_MovementSpeed Enum" :default "NewEnumerator0"))
  (bind _charactermovement (`self.CharacterMovement`))
  (if (`|EnumInequality` NewSpeedMode (`self.MovementSpeedMode`))
    (bind _output_get (set `self.MovementSpeedMode` NewSpeedMode))
    (switch `/Game/CombatSystem/Blueprints/Enum/E_MovementSpeed` _output_get
      (:`NewEnumerator0`
        (set `CharacterMovementComponent.MaxWalkSpeed` (`self.Walk Speed`) _charactermovement))
      (:`NewEnumerator1`
        (set `CharacterMovementComponent.MaxWalkSpeed` (`self.Run Speed`) _charactermovement))
      (:`NewEnumerator2`
        (set `CharacterMovementComponent.MaxWalkSpeed` (`self.Sprint Speed`) _charactermovement)))))

(fn `UserConstructionScript`)