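; Base weapon actor for the combat system, equippable on body or in hand, with montages mapped to action gameplay tags.
; A state manager component tracks on-body, in-hand and physics-simulated states.
; Collision component hits apply point damage using unscaled WeaponBaseDamage to actors accepting damage messages.
; Separate getters derive damage, cost and cost type from the owner's current action; collision activate/deactivate functions are empty.
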(event `self.CollisionComponent.OnHit`
  (params (`Hit Result` :type "HitResult Structure"))
  (bind (_bblockinghit _binitialoverlap _time _distance _location _impactpoint _normal _impactnormal _physmat _hitactor) (`GameplayStatics.BreakHitResult` `Hit Result`))
  (bind _canreceivedamage_ (message `/Game/CombatSystem/Blueprints/Interface/BPI_Combat.CanReceiveDamage` _hitactor))
  (if _canreceivedamage_
    (`GameplayStatics.ApplyPointDamage` _hitactor (`self.WeaponBaseDamage`) (`self.GetActorForwardVector` (`self.GetOwner`)) `Hit Result` (`self.GetInstigatorController`) self (`self.Damage Type Class`))))

(event `SimulateWeaponPhysics`
  (bind _return_value (`self.GetItemMesh`))
  (`PrimitiveComponent.SetCollisionProfileName` _return_value "PhysicsActor" true)
  (`PrimitiveComponent.SetSimulatePhysics` _return_value true)
  (`/Game/CombatSystem/Blueprints/Components/BPC_StateManagerComponent.SetCurrentState` (`self.BPC_StateManagerComponent`) (struct :`TagName` "Weapon.State.SimulatingPhysics")))

(fn `ActivateCollision`
  (params (CollisionPart :type "/Game/CombatSystem/Blueprints/Enum/E_CollisionPart Enum" :default "NewEnumerator0")))

(fn `DeactiveCollision`
  (params (CollisionPart :type "/Game/CombatSystem/Blueprints/Enum/E_CollisionPart Enum" :default "NewEnumerator0")))

(fn `EquipeOnBody`
  (`parent.EquipeOnBody`)
  (`/Game/CombatSystem/Blueprints/Components/BPC_StateManagerComponent.SetCurrentState` (`self.BPC_StateManagerComponent`) (struct :`TagName` "Weapon.State.OnBody"))
  (set `self.StatesManager` (`self.GetComponentByClass` (`self.GetOwner`) "/Game/CombatSystem/Blueprints/Components/BPC_StateManagerComponent.BPC_StateManagerComponent_C"))
  (`/Game/CombatSystem/Blueprints/Components/BPC_CollisionComponent.SetCollisionMesh` (`self.CollisionComponent`) (`self.GetItemMesh`))
  (`/Game/CombatSystem/Blueprints/Components/BPC_CollisionComponent.AddActorToIgnore` (`self.CollisionComponent`) (`self.GetOwner`)))

(fn `EquipeOnHand`
  (`/Game/CombatSystem/Blueprints/Components/BPC_StateManagerComponent.SetCurrentState` (`self.BPC_StateManagerComponent`) (struct :`TagName` "Weapon.State.OnHand"))
  (`self.SetIsEquipeOnBody` false)
  (`self.AttachActor` (`self.WeaponHandSocket`)))

(fn `Find Weapon Montage`
  (params (CharacterAction :type "GameplayTag Structure"))
  (returns (EquipeMontage :type "Array of AnimMontage Object Reference"))
  (`|SwitchGameplayTag` CharacterAction
    (:`Default`
      (return))
    (:`Character.Action.Attack.NormalAttack`
      (return (`self.NormalAttack`)))
    (:`Character.Action.Attack.SpecialAttack`
      (return (`|MakeArray` (`self.SpecialAttack`))))
    (:`Character.Action.Attack.ChargedAttack`
      (return (`self.ChargedAttack`)))
    (:`Character.Action.Attack.FallingAttack`
      (return (`self.FallingAttack`)))
    (:`Character.Action.Attack.SprintAttack`
      (return (`|MakeArray` (`self.SprintAttck`))))
    (:`Character.Action.Dodge`
      (return (`self.DodgeMontage`)))
    (:`Character.Action.DisarmWeapon`
      (return (`|MakeArray` (`self.DisarmMontage`))))
    (:`Character.Action.DrawWeapon`
      (return (`|MakeArray` (`self.DrawMontage`))))))

(fn `GetActionCost`
  (returns (Value :type "Float (double-precision)"))
  (bind _statesmanager (`self.StatesManager`)
    (:`then`
      (return (`BlueprintMapLibrary.Map_Find` (`self.ActionCost`) (`/Game/CombatSystem/Blueprints/Components/BPC_StateManagerComponent.GetCurrentAction` _statesmanager))))
    (:`else`
      (return 0.0))))

(fn `GetActionCostType`
  (returns (CostType :type "/Game/CombatSystem/Blueprints/Enum/E_Stats Enum"))
  (bind _statesmanager (`self.StatesManager`)
    (:`then`
      (return (`BlueprintMapLibrary.Map_Find` (`self.ActionStatCostType`) (`/Game/CombatSystem/Blueprints/Components/BPC_StateManagerComponent.GetCurrentAction` _statesmanager))))
    (:`else`
      (return "NewEnumerator0"))))

(fn `GetActionDamage`
  (returns (Damage :type "Float (double-precision)"))
  (bind _statesmanager (`self.StatesManager`)
    (:`then`
      (return (* (`self.WeaponBaseDamage`) (`BlueprintMapLibrary.Map_Find` (`self.ActionDamageMultiplier`) (`/Game/CombatSystem/Blueprints/Components/BPC_StateManagerComponent.GetCurrentAction` _statesmanager)))))
    (:`else`
      (return (`self.WeaponBaseDamage`)))))

(fn `IsWeaponOnHand`
  (returns (`isWeaponOnHand?` :type Boolean))
  (if (`self.IsEquipeOnBody`)
    (return false)
    (else
      (return true))))

(fn `UserConstructionScript`
  (`parent.UserConstructionScript`))