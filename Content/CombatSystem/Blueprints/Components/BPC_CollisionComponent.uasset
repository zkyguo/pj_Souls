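; Combat collision component that detects hits along a socketed mesh, likely a weapon, and fires OnHit.
; CollisionTrace runs a multi-sphere object trace between start and end sockets, skipping ignored actors and reporting each actor once until the hit list clears.
; EnableCollision clears that list and raises the enabled flag.
; As written, Tick only resets that flag, and nothing here calls CollisionTrace.
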(event `CollisionTrace`
  (bind _collisionmeshcomponent (`self.CollisionMeshComponent`))
  (bind _alreadyhitactor (`self.AlreadyHitActor`))
  ;[1 1 1] Collision Trace
  (bind _outhits (`KismetSystemLibrary.SphereTraceMultiForObjects` (`SceneComponent.GetSocketLocation` _collisionmeshcomponent (`self.StartSocketName`)) (`SceneComponent.GetSocketLocation` _collisionmeshcomponent (`self.EndSocketName`)) (`self.TraceRadius`) (`self.CollisiojnObject Types`) false (`self.Actors to Ignore`) (`self.Draw Debug Type`)))
  (for _array_element _outhits
    (bind _output_get (set `self.LastHit` _array_element))
    (bind (_bblockinghit _binitialoverlap _time _distance _location _impactpoint _normal _impactnormal _physmat _hitactor) (`GameplayStatics.BreakHitResult` _output_get))
    (if (not (`KismetArrayLibrary.Array_Contains` _alreadyhitactor _hitactor))
      (bind _output_get_2 (set `self.Hit Actor` _hitactor))
      (`KismetArrayLibrary.Array_Add` _alreadyhitactor _output_get_2)
      (`self.OnHit` (`self.LastHit`)))))

(event `self.ReceiveTick`
  (params (DeltaSeconds :type "Float (single-precision)"))
  (if (`self.IsCollisionEnable?`)
    (set `self.IsCollisionEnable?` false)))

(event `EnableCollision`
  (`self.ClearHitActor`)
  (set `self.IsCollisionEnable?` true))

(event `Disable Collision`
  (set `self.IsCollisionEnable?` false))

(event `ClearHitActor`
  (`KismetArrayLibrary.Array_Clear` (`self.AlreadyHitActor`)))

(event `SetCollisionMesh`
  (params (MeshComponent :type "PrimitiveComponent Object Reference"))
  (set `self.CollisionMeshComponent` MeshComponent))

(fn `AddActorToIgnore`
  (params (Actor :type "Actor Object Reference (by ref)"))
  (`KismetArrayLibrary.Array_AddUnique` (`self.Actors to Ignore`) Actor))

(fn `GetActorToIgnore`
  (returns (`Actors to Ignore` :type "Array of Actor Object Reference"))
  (return (`self.Actors to Ignore`)))

(fn `GetAlreadyHitActor`
  (returns (AlreadyHitActor :type "Array of Actor Object Reference"))
  (return (`self.AlreadyHitActor`)))

(fn `GetCollisionMeshComponent`
  (returns (NewParam :type "PrimitiveComponent Object Reference"))
  (return (`self.CollisionMeshComponent`)))

(fn `GetLastHit`
  (returns (LastHit :type "HitResult Structure"))
  (return (`self.LastHit`)))

(fn `IsCollisionEnabled?`
  (returns (`IsCollisionEnable?` :type Boolean))
  (return (`self.IsCollisionEnable?`)))

(fn `RemoveActorToIgnore`
  (params (Actor :type "Actor Object Reference (by ref)"))
  (`KismetArrayLibrary.Array_RemoveItem` (`self.Actors to Ignore`) Actor))