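; Actor component that manages combat stats such as health, stamina and armor, including damage and death.
; Base stats seed a current-value map, and each change broadcasts an update.
; Clamped updates restart regeneration: health and stamina use looping timers behind a retriggerable delay, paused at max.
; TakeDamage scales damage against armor; at zero health it sets the Dead state, stops health regen and clears owner targeting.
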(event `StartRegen`
  (params (`Stat ` :type "/Game/CombatSystem/Blueprints/Enum/E_Stats Enum" :default "NewEnumerator0"))
  (switch `/Game/CombatSystem/Blueprints/Enum/E_Stats` `Stat `
    (:`NewEnumerator1`
      (`KismetSystemLibrary.K2_ClearTimer` null "RegenHealth")
      (`KismetSystemLibrary.RetriggerableDelay` 0.2)
      (bind _returnvalue (`KismetSystemLibrary.K2_SetTimer` null "RegenHealth" 0.1 true)))
    (:`NewEnumerator2`
      (`KismetSystemLibrary.K2_ClearTimer` null "RegenStamina")
      (`KismetSystemLibrary.RetriggerableDelay` 0.2)
      (bind _returnvalue_2 (`KismetSystemLibrary.K2_SetTimer` null "RegenStamina" 0.1 true)))))

(event `RegenStamina`
  (`self.RegenStatValue` "NewEnumerator2"))

(event `RegenHealth`
  (`self.RegenStatValue` "NewEnumerator1"))

(event `StopRegen`
  (params (Selection :type "/Game/CombatSystem/Blueprints/Enum/E_Stats Enum" :default "NewEnumerator0"))
  (switch `/Game/CombatSystem/Blueprints/Enum/E_Stats` Selection
    (:`NewEnumerator1`
      (`KismetSystemLibrary.K2_PauseTimerHandle` (stale `StartRegen` _returnvalue)))
    (:`NewEnumerator2`
      (`KismetSystemLibrary.K2_PauseTimerHandle` (stale `StartRegen` _returnvalue_2)))))

(fn `GetBaseStatValue`
  (params (Stat :type "/Game/CombatSystem/Blueprints/Enum/E_Stats Enum" :default "NewEnumerator0"))
  (returns (`Base Value` :type "Float (double-precision)"))
  (return (break `/Game/CombatSystem/Blueprints/Struct/F_BaseRegenStat` (`BlueprintMapLibrary.Map_Find` (`self.BaseStats`) Stat))))

(fn `GetCurrentStatValue`
  (params (Stat :type "/Game/CombatSystem/Blueprints/Enum/E_Stats Enum" :default "NewEnumerator0"))
  (returns (Value :type "Float (double-precision)"))
  (return (`BlueprintMapLibrary.Map_Find` (`self.CurrentStats`) Stat)))

(fn `GetMaxStatValue`
  (params (Stat :type "/Game/CombatSystem/Blueprints/Enum/E_Stats Enum" :default "NewEnumerator0"))
  (returns (`Max Value` :type "Float (double-precision)"))
  (return (`.MaxValue_4_2EA803B34DB27E398D48A9A123683B73` (break `/Game/CombatSystem/Blueprints/Struct/F_BaseRegenStat` (`BlueprintMapLibrary.Map_Find` (`self.BaseStats`) Stat)))))

(fn `GetStatRegenRate`
  (params (Stat :type "/Game/CombatSystem/Blueprints/Enum/E_Stats Enum" :default "NewEnumerator0"))
  (returns (`Regen Rate` :type "Float (double-precision)"))
  (return (`.RegenRate_7_8350F50D49951BFD8CA816A3D112C08E` (break `/Game/CombatSystem/Blueprints/Struct/F_BaseRegenStat` (`BlueprintMapLibrary.Map_Find` (`self.BaseStats`) Stat)))))

(fn `InitializaStats`
  (bind _basestats (`self.BaseStats`))
  (bind _keys (`BlueprintMapLibrary.Map_Keys` _basestats))
  (for _array_element _keys
    (bind (_basevalue _maxvalue _regenrate) (break `/Game/CombatSystem/Blueprints/Struct/F_BaseRegenStat` (`BlueprintMapLibrary.Map_Find` _basestats _array_element)))
    (`self.SetCurrentStatValue` _array_element _basevalue)
    (`self.SetStatRegenRate` _array_element _regenrate)))

(fn `RegenStatValue`
  (params (Stat :type "/Game/CombatSystem/Blueprints/Enum/E_Stats Enum" :default "NewEnumerator0"))
  (`self.UpdateCurrentStats` Stat (`self.GetStatRegenRate` Stat))
  (if (>= (`self.GetCurrentStatValue` Stat) (`self.GetMaxStatValue` Stat))
    (`self.StopRegen` Stat)))

(fn `SetBaseStatValue`
  (params (Stat :type "/Game/CombatSystem/Blueprints/Enum/E_Stats Enum" :default "NewEnumerator0") (` Value` :type "Float (double-precision)"))
  (bind _basestats (`self.BaseStats`))
  (bind _structout (setmembers `/Game/CombatSystem/Blueprints/Struct/F_BaseRegenStat` :`StructRef` (`BlueprintMapLibrary.Map_Find` _basestats Stat) :`BaseValue` ` Value`))
  (`BlueprintMapLibrary.Map_Add` _basestats Stat _structout))

(fn `SetCurrentStatValue`
  (params (Stat :type "/Game/CombatSystem/Blueprints/Enum/E_Stats Enum" :default "NewEnumerator0") (Value :type "Float (double-precision) (by ref)"))
  (`BlueprintMapLibrary.Map_Add` (`self.CurrentStats`) Stat Value)
  (`self.OnCurrentStatValueUpdate` Value Stat))

(fn `SetMaxStatValue`
  (params (Stat :type "/Game/CombatSystem/Blueprints/Enum/E_Stats Enum" :default "NewEnumerator0") (MaxValue :type "Float (double-precision)"))
  (bind _basestats (`self.BaseStats`))
  (bind _structout (setmembers `/Game/CombatSystem/Blueprints/Struct/F_BaseRegenStat` :`StructRef` (`BlueprintMapLibrary.Map_Find` _basestats Stat) :`MaxValue` MaxValue))
  (`BlueprintMapLibrary.Map_Add` _basestats Stat _structout))

(fn `SetStatRegenRate`
  (params (Stat :type "/Game/CombatSystem/Blueprints/Enum/E_Stats Enum" :default "NewEnumerator0") (` Value` :type "Float (double-precision)"))
  (bind _basestats (`self.BaseStats`))
  (bind _structout (setmembers `/Game/CombatSystem/Blueprints/Struct/F_BaseRegenStat` :`StructRef` (`BlueprintMapLibrary.Map_Find` _basestats Stat) :`Regen Rate` ` Value`))
  (`BlueprintMapLibrary.Map_Add` _basestats Stat _structout))

(fn `TakeDamage`
  (params (InDamage :type "Float (double-precision)" :default 0.0))
  (locals (FinalDamage :type "Float (double-precision)"))
  (bind _returnvalue (`self.GetOwner`))
  (bind _returnvalue_2 (* (`local.InDamage`) (/ (`local.InDamage`) (+ (`local.InDamage`) (`self.GetCurrentStatValue` "NewEnumerator4")))))
  (bind _output_get (set `local.FinalDamage` (`KismetMathLibrary.FClamp` _returnvalue_2 0.0 _returnvalue_2)))
  (`KismetSystemLibrary.PrintString` (`KismetStringLibrary.Conv_DoubleToString` _output_get))
  (`self.UpdateCurrentStats` "NewEnumerator1" (* _output_get -1.0))
  (if (<= (`self.GetCurrentStatValue` "NewEnumerator1") 0.0)
    (`/Game/CombatSystem/Blueprints/Components/BPC_StateManagerComponent.SetCurrentState` (`Actor.GetComponentByClass` _returnvalue "/Game/CombatSystem/Blueprints/Components/BPC_StateManagerComponent.BPC_StateManagerComponent_C") (struct :`TagName` "Character.State.Dead"))
    (`self.StopRegen` "NewEnumerator1")
    (message `/Game/CombatSystem/Blueprints/Interface/BPI_Targeting.OnTargeted` _returnvalue false)))

(fn `UpdateCurrentStats`
  (params (Stat :type "/Game/CombatSystem/Blueprints/Enum/E_Stats Enum" :default "NewEnumerator0") (Value :type "Float (double-precision)"))
  (locals (Loacal_Value :type "Float (double-precision)"))
  (bind _stat (`local.Stat`))
  (if (!= Value 0.0)
    (bind _output_get (set `local.Loacal_Value` (+ (`self.GetCurrentStatValue` (`local.Stat`)) (`local.Value`))))
    (bind _output_get_2 (set `local.Loacal_Value` (`KismetMathLibrary.FClamp` _output_get 0.0 (`self.GetMaxStatValue` (`local.Stat`)))))
    (`self.SetCurrentStatValue` _stat _output_get_2)
    (`self.StartRegen` _stat)))