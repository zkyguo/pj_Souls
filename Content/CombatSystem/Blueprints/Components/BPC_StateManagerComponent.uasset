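; Actor component in the combat system that tracks a character's current state and current action as Gameplay Tags.
; Setters act only when the value changes, calling end events for the old tag and begin events for the new one.
; Exact-match checks test both values against tag containers, and ResetState picks GeneralAction or None based on whether a weapon is in hand.
; Tick prints both current tags for debugging.
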(event `self.ReceiveTick`
  (params (DeltaSeconds :type "Float (single-precision)"))
  (`KismetSystemLibrary.PrintString` (`KismetStringLibrary.Concat_StrStr` "Current State :" (`KismetStringLibrary.Conv_NameToString` (`BlueprintGameplayTagLibrary.GetTagName` (`self.CurrentState`)))) true true (struct :`G` 0.66 :`B` 1.0 :`A` 1.0) 0.0)
  (`KismetSystemLibrary.PrintString` (`KismetStringLibrary.Concat_StrStr` "Current Action :" (`KismetStringLibrary.Conv_NameToString` (`BlueprintGameplayTagLibrary.GetTagName` (`self.CurrentCharacterAction`)))) true true (struct :`G` 0.66 :`B` 1.0 :`A` 1.0) 0.0))

(fn `GetCurrentAction`
  (returns (CurrentCharacterAction :type "GameplayTag Structure"))
  (return (`self.CurrentCharacterAction`)))

(fn `GetCurrentState`
  (returns (CurrentState :type "GameplayTag Structure"))
  (return (`self.CurrentState`)))

(fn `IsCurrentActionEqualTo?`
  (params (ActionToCheck :type "GameplayTagContainer Structure" :default (struct :`GameplayTags` (struct :`(TagName` "Character.Action.Attack.ChargedAttack") :`(TagName` "Character.Action.Attack.FallingAttack") :`(TagName` "Character.Action.Attack.NormalAttack") :`(TagName` "Character.Action.Attack.SpecialAttack") :`(TagName` "Character.Action.Attack.SprintAttack") :`(TagName` "Character.Action.DisarmWeapon") :`(TagName` "Character.Action.Dodge") :`(TagName` "Character.Action.DrawWeapon") :`(TagName` "Character.Action.Nothing")))))
  (returns (`IsCurrentActionEqualTo?` :type Boolean))
  (return (`BlueprintGameplayTagLibrary.HasTag` ActionToCheck (`self.CurrentCharacterAction`) true)))

(fn `IsCurrentStateEqualTo?`
  (params (StateToCheck :type "GameplayTagContainer Structure" :default (struct :`GameplayTags` (struct :`(TagName` "Character.State.Attacking") :`(TagName` "Character.State.Dead") :`(TagName` "Character.State.Disable") :`(TagName` "Character.State.Dodging") :`(TagName` "Character.State.General Action") :`(TagName` "Character.State.None")))))
  (returns (`IsCurrentStateEqualTo?` :type Boolean))
  (return (`BlueprintGameplayTagLibrary.HasTag` StateToCheck (`self.CurrentState`) true)))

(fn `ResetState`
  (params (`WeaponOnHand?` :type Boolean))
  (if `WeaponOnHand?`
    (`self.SetCurrentState` (struct :`TagName` "Character.State.General Action"))
    (else
      (`self.SetCurrentState` (struct :`TagName` "Character.State.None")))))

(fn `SetCurrentAction`
  (params (NewAction :type "GameplayTag Structure"))
  (bind _currentcharacteraction (`self.CurrentCharacterAction`))
  (if (!= _currentcharacteraction NewAction)
    (`self.OnCharacterActionEnd` _currentcharacteraction)
    (bind _output_get (set `self.CurrentCharacterAction` (`local.NewAction`)))
    (`self.OnCharacterActionBegin` _output_get)))

(fn `SetCurrentState`
  (params (NewState :type "GameplayTag Structure"))
  (if (!= (`self.CurrentState`) NewState)
    (`self.OnStateEnd` (`self.CurrentState`))
    (bind _output_get (set `self.CurrentState` (`local.NewState`)))
    (`self.OnStateBegin` _output_get)
    (return)))