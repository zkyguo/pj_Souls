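; BPC_CombatComponent is an actor component that holds and swaps the main weapon of BP_Playerharacter, its owner cached on BeginPlay.
; SetMainWeapon records whether the old weapon was on the body, destroys it, then equips the new one in that same body or hand slot, defaulting to body.
; It also messages the player's AnimInstance with the weapon's type when in hand, or a fixed combat type when on the body.
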(event `self.ReceiveBeginPlay`
  (bind _asbp_playerharacter (cast `/Game/CombatSystem/Blueprints/BP_Playerharacter` (`self.GetOwner`)))
  (set `self.Player` _asbp_playerharacter))

(fn `GetMainWeapon`
  (returns (MainWeapon :type "/Game/CombatSystem/Blueprints/Actors/BP_BaseWeapon Object Reference"))
  (return (`self.MainWeapon`)))

(fn `SetMainWeapon`
  (params (NewWeapon :type "/Game/CombatSystem/Blueprints/Actors/BP_BaseWeapon Object Reference"))
  (locals (IsUnequipe :type Boolean))
  (bind _mainweapon (`self.MainWeapon`))
  (bind _mainweapon_2 (`self.MainWeapon`))
  (bind _returnvalue (`SkeletalMeshComponent.GetAnimInstance` (`Character.Mesh` (`self.Player`))))
  (`|ExecutionSequence`
    (:`then_0`
      (`/Engine/EditorBlueprintResources/StandardMacros.IsValid` _mainweapon
        (:`Is Valid`
          (set `local.IsUnequipe` (`/Game/CombatSystem/Blueprints/Actors/BP_BaseEquippable.IsEquipeOnBody` _mainweapon))
          (`Actor.K2_DestroyActor` _mainweapon))
        (:`Is Not Valid`
          (set `local.IsUnequipe` true))))
    (:`then_1`
      (bind _output_get (set `self.MainWeapon` NewWeapon))
      (if (`local.IsUnequipe`)
        (message `/Game/CombatSystem/Blueprints/Interface/BPI_AnimationInstance.UpdateCombatType` _returnvalue "NewEnumerator3")
        (`/Game/CombatSystem/Blueprints/Actors/BP_BaseEquippable.EquipeOnBody` _mainweapon_2)
        (else
          (message `/Game/CombatSystem/Blueprints/Interface/BPI_AnimationInstance.UpdateCombatType` _returnvalue (`/Game/CombatSystem/Blueprints/Actors/BP_BaseWeapon.WeaponType` _output_get))
          (`/Game/CombatSystem/Blueprints/Actors/BP_BaseWeapon.EquipeOnHand` _mainweapon_2))))))